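; BP_Player_Base is the player's base, which costs the player a life whenever an enemy reaches it.
; On overlap with a BP_Enemy, it destroys that enemy and decrements Lives on NewGameMode.
; It then finds the BP_Spawner by class and decrements its ExistingEnemies count.
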(event EventBeginPlay)

(event Collision|EventActorBeginOverlap
  (params (OtherActor :type Actor%20Object%20Reference))
  (bind _asbp_enemy (Utilities|Casting|CastToBP_Enemy OtherActor))
  (Utilities|FlowControl|Sequence
    (:then_0
      (Actor|DestroyActor _asbp_enemy))
    (:then_1
      (bind _asnew_game_mode (Utilities|Casting|CastToNewGameMode (Game|GetGameMode)))
      (Variables|/Game/Blueprints/GameSettings/NewGameMode.NewGameMode_C|SetLives _asnew_game_mode (- (Variables|/Game/Blueprints/GameSettings/NewGameMode.NewGameMode_C|GetLives _asnew_game_mode) 1)))
    (:then_2
      (bind _returnvalue (Actor|GetActorOfClass "/Game/Blueprints/World/BP_Spawner.BP_Spawner_C"))
      (Variables|/Game/Blueprints/World/BP_Spawner.BP_Spawner_C|SetExisting_enemies _returnvalue (- (Variables|/Game/Blueprints/World/BP_Spawner.BP_Spawner_C|GetExisting_enemies _returnvalue) 1)))))

(event EventTick
  (params (DeltaSeconds :type Float%20%28single-precision%29)))

(fn ConstructionScript)