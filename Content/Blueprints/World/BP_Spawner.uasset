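; BP_Spawner is a wave spawner that creates enemies at its own location, scaled to the game mode's current wave.
; Spawn_enemy runs delayed loops for the first ZombieClass type and, on later waves, a second type, with counts growing per wave.
; Both share one spawn chain that counts enemies, creates their controllers and adds wave-based health.
; The start delay and wave-increment logic is disconnected and never runs.
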(event Custom|Spawn_enemy
  ;[1 1 1] Switcher between enemies depending on current level
  (Variables|Default|SetCurrent_Wave (Variables|/Game/Blueprints/GameSettings/NewGameMode.NewGameMode_C|GetCurent_Wave (Variables|Default|GetGameMode)))
  (Utilities|FlowControl|Sequence
    (:then_0
      (Utilities|ForLoopwithDelay 1 (* (Variables|Default|GetCurrent_Wave) (Variables|Default|GetEnemiesPerLevel)) 0.6
        (:LoopBody
          (Variables|Default|SetSwitcher 0)
          ;[1 1 1] Enemy Spawner
          (Utilities|FlowControl|Sequence :!label _label
            (:then_0
              (Variables|Default|SetExisting_enemies (+ (Variables|Default|GetExisting_enemies) 1)))
            (:then_1
              (bind _returnvalue (Game|SpawnActorfromClass (Utilities|Array|Get(acopy) (Variables|Default|GetZombie_Class) (Variables|Default|GetSwitcher)) (Math|Conversions|ToTransform(Vector) (Transformation|GetActorLocation self)) "AdjustIfPossibleButAlwaysSpawn" 0 0))
              ;[1 1 1] Increase the health for spawned enemies for each level
              (bind _output_get (Variables|Default|SetSpawned_Enemy _returnvalue))
              (bind _asbp_enemy (Utilities|Casting|CastToBP_Enemy _output_get))
              (Pawn|SpawnDefaultController _asbp_enemy)
              (Variables|/Game/Blueprints/ThirdPersonBP/Blueprints/BP_Enemy.BP_Enemy_C|SetHealth _asbp_enemy (+ (Variables|/Game/Blueprints/ThirdPersonBP/Blueprints/BP_Enemy.BP_Enemy_C|GetHealth _asbp_enemy) (Math|Conversions|ToFloat(Integer) (* (Variables|/Game/Blueprints/GameSettings/NewGameMode.NewGameMode_C|GetCurent_Wave (Variables|Default|GetGameMode)) 10)))))))))
    (:then_1
      (if (> (Variables|Default|GetCurrent_Wave) 2)
        (Utilities|ForLoopwithDelay 1 (* (Variables|Default|GetCurrent_Wave) 2) 1.0
          (:LoopBody
            (Variables|Default|SetSwitcher 1)
            (goto _label)))))))

(event EventBeginPlay
  (Utilities|FlowControl|Sequence
    (:then_0
      (bind _asnew_game_mode (Utilities|Casting|CastToNewGameMode (Game|GetGameMode)))
      (Variables|Default|SetGameMode _asnew_game_mode))
    (:then_1
      (Utilities|Casting|CastToBP_Enemy (Components|GetOwner)))))

(fn ConstructionScript)