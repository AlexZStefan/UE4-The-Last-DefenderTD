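; Behavior Tree task that writes spline point world locations to a Blackboard vector key.
; It casts the owner actor to Splines and loops over every point of its spline, overwriting the BBRef key each time.
; FinishExecute(true) is called inside the loop body rather than after it, and a failed cast never finishes the task.
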(event EventReceiveExecute
  (params (OwnerActor :type Actor%20Object%20Reference))
  (bind _assplines (Utilities|Casting|CastToSplines OwnerActor))
  (Variables|Default|SetSplines _assplines)
  (for _index (range 0 (- (Spline|GetNumberOfSplinePoints (Variables|/Game/data/Splines.Splines_C|GetSpline _assplines)) 1))
    (AI|BehaviorTree|SetBlackboardValueasVector (Variables|Default|GetBB_Ref) (Spline|GetLocationatSplinePoint (Variables|/Game/data/Splines.Splines_C|GetSpline (Variables|Default|GetSplines)) _index "World"))
    (AI|BehaviorTree|FinishExecute true)))