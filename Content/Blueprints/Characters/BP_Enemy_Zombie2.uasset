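; BP_Enemy_Zombie2 is a zombie enemy Blueprint that plays a hit reaction when a projectile overlaps its capsule.
; Capsule overlap sets GotHit, then a Sequence casts the other actor to the standard, fire and slowC projectile classes.
; A successful cast plays the GetHit section of the Zombie_strong_actions montage, and ending the overlap clears GotHit.
; BeginPlay and construction defer to the parent, and no damage is applied here.
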(event OnComponentBeginOverlap(CapsuleComponent)
  (params (OverlappedComponent :type Primitive%20Component%20Object%20Reference) (OtherActor :type Actor%20Object%20Reference) (OtherComp :type Primitive%20Component%20Object%20Reference) (OtherBodyIndex :type Integer) (bFromSweep :type Boolean) (SweepResult :type Hit%20Result%20Structure%20%28by%20ref%29))
  (bind _output_get (Variables|Default|SetgotHit? true))
  (if _output_get
    (Utilities|FlowControl|Sequence
      (:then_0
        (Utilities|Casting|CastToBP_Projectile OtherActor))
      (:then_1
        (Utilities|Casting|CastToBP_Projectile_fire OtherActor))
      (:then_2
        (Utilities|Casting|CastToBP_Projectile_slowC OtherActor)))
    (Animation|PlayAnimMontage "/Game/Blueprints/Characters/StrongZombie/Animations/Zombie_strong_actions.Zombie_strong_actions" 1.0 "GetHit")))

(event OnComponentEndOverlap(CapsuleComponent)
  (params (OverlappedComponent :type Primitive%20Component%20Object%20Reference) (OtherActor :type Actor%20Object%20Reference) (OtherComp :type Primitive%20Component%20Object%20Reference) (OtherBodyIndex :type Integer))
  (Variables|Default|SetgotHit? false))

(event EventBeginPlay
  (|CallParentFunction))

(event Collision|EventActorBeginOverlap
  (params (OtherActor :type Actor%20Object%20Reference)))

(event EventTick
  (params (DeltaSeconds :type Float%20%28single-precision%29))
  (|CallParentFunction DeltaSeconds) ; This node is disabled and will not be called.\nDrag off pins to build functionality.
)

(fn ConstructionScript
  (|CallParentFunction))