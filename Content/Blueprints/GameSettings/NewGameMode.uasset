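; NewGameMode is the game mode for a wave-based game, managing wave progression and game over.
; BeginPlay caches the player and spawner, shows the HUD, then starts the game after a delay.
; Tick polls the spawner's living enemy count, waiting before incrementing the wave and spawning again.
; When lives run out, Tick swaps the HUD for a game-over widget, shows the cursor, pauses and plays a sound.
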(event EventBeginPlay
  (Utilities|FlowControl|Sequence
    (:then_0
      (bind _asbp_player (Utilities|Casting|CastToBP_Player (Game|GetPlayerCharacter 0)))
      (Variables|Default|SetPlayer _asbp_player))
    (:then_1
      (bind _asbp_enemy (Utilities|Casting|CastToBP_Enemy (Components|GetOwner))))
    (:then_3
      (bind _returnvalue (Actor|GetActorOfClass "/Game/Blueprints/World/BP_Spawner.BP_Spawner_C"))
      (bind _asbp_spawner (Utilities|Casting|CastToBP_Spawner _returnvalue))
      (Variables|Default|SetSpawner _asbp_spawner))
    (:then_4
      ;[1 1 1] PlayerUI
      (bind _returnvalue_2 (UserInterface|CreateWidget "/Game/Blueprints/UI/Widget_UI.Widget_UI_C"))
      (bind _output_get (Variables|Default|SetUserUI _returnvalue_2))
      (UserInterface|Viewport|AddtoViewport _output_get 0)
      (Utilities|FlowControl|Delay 15.0) ; Delay before first wave spawn
      (Variables|Default|SetGameStart true))))

(event EventTick
  (params (DeltaSeconds :type Float%20%28single-precision%29))
  (bind _spawner (Variables|Default|GetSpawner))
  (Utilities|FlowControl|Sequence
    (:then_0
      ;[1 1 1] Player Defeat
      (if (<= (Variables|Default|GetLives) 0)
        (Variables|Default|SetGameOver true)
        (Widget|SetVisibility (Variables|Default|GetUserUI) "Hidden")
        (bind _returnvalue (UserInterface|CreateWidget "/Game/Blueprints/UI/WG_GameOver.WG_GameOver_C"))
        (UserInterface|Viewport|AddtoViewport _returnvalue 0)
        (Variables|/Script/Engine.PlayerController|SetbShowMouseCursor (Game|GetPlayerController 0) true)
        (Utilities|FlowControl|DoN 1
          (:Exit
            (Game|SetGamePaused true)
            (Audio|PlaySound2D "/Game/Sounds/FinishedLevel.FinishedLevel" 1.0 1.0 0.0 0 0)))))
    (:then_2
      (if (Variables|Default|GetGameStart)
        ;[1 1 1] Spawn Enemies and increase the level after all enemies defeted
        (if (<= (Variables|/Game/Blueprints/World/BP_Spawner.BP_Spawner_C|GetExisting_enemies (Variables|Default|GetSpawner)) 0)
          (Utilities|FlowControl|Sequence
            (:then_0
              (Utilities|FlowControl|Delay 15.0) ; Delay Bofore Spawn
              (if (<= (Variables|/Game/Blueprints/World/BP_Spawner.BP_Spawner_C|GetExisting_enemies (Variables|Default|GetSpawner)) 0)
                (Variables|/Game/Blueprints/World/BP_Spawner.BP_Spawner_C|SetExisting_enemies _spawner 0)
                (Variables|Default|SetCurent_Wave (+ (Variables|Default|GetCurent_Wave) 1))
                (Default|SpawnEnemy _spawner)))))))))

(fn ConstructionScript)