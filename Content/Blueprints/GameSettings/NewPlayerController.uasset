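; Player controller for a tower defense game, handling projectile firing, tower building, upgrading and selling with coins, and the pause menu.
; Tower keys spawn a tinted, collision-free preview that Tick moves along a camera trace, with rotation and snapping beside existing towers.
; A downward trace detects build locations and charges coins on placement.
; Upgrade and sell trace from the camera; upgrade cost scales with level, capped at three.
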(event Custom|Upgrade_Tower
  ;[1 1 1] Upgrade tower
)

(event Custom|ResumeGame
  ;[1 1 1] PauseMenu
  (CallFunction|ToogleMenu))

(event EventBeginPlay
  ;[1 1 1] Casting
  (Utilities|FlowControl|Sequence
    (:then_0
      (bind _asbp_player (Utilities|Casting|CastToBP_Player (Game|GetPlayerCharacter 0)))
      (Variables|Default|SetPlayerCharacter _asbp_player))
    (:then_1
      (bind _asnew_game_mode (Utilities|Casting|CastToNewGameMode (Game|GetGameMode)))
      (Variables|Default|SetGameMode _asnew_game_mode))))

(event EventTick
  (params (DeltaSeconds :type Float%20%28single-precision%29))
  (bind _being_build (Variables|Default|GetBeing%20Build))
  (bind _staticmesh (Variables|/Game/Blueprints/Turrets/BP_Tower.BP_Tower_C|GetStaticMesh _being_build))
  ;[1 1 1] Builds the turret
  (if (Variables|Default|GetIsBuilding?)
    (CallFunction|PositionPath) ; Adjust the location of where to build
    (if (Variables|Default|GetClickToPlace)
      (Variables|Default|SetClickToPlace false)
      (Collision|SetCollisionEnabled _staticmesh "QueryAndPhysics")
      (Rendering|Material|SetVectorParameterValueonMaterials _staticmesh "Tint" "1.000000,1.000000,1.000000") ; Changes the mat col. when placed
      (Collision|SetCollisionObjectType (Variables|/Game/Blueprints/Turrets/BP_Tower.BP_Tower_C|GetTurretProj _being_build) "ECC_GameTraceChannel2")
      (bind _returnvalue (Actor|GetActorOfClass "/Game/Blueprints/Turrets/BP_Tower.BP_Tower_C"))
      (CallFunction|SpawnBuildItem)
      (Variables|/Game/Blueprints/Turrets/BP_Tower.BP_Tower_C|SetTower_Level _returnvalue 1)
      (Variables|Default|SetIsBuilding? false)
      (Audio|PlaySound2D "/Game/Sounds/build.build" 1.0 1.0 0.0 0 0))))

(event Input|ActionEvents|InputActionPlaceBuildItem
  (params (Key :type Key%20Structure :default "None"))
  ;[1 1 1] rotate building
  (:Pressed
    (Variables|Default|SetClickToPlace true)))

(event Input|ActionEvents|InputActionRotatePart
  (params (Key :type Key%20Structure :default "None"))
  ;[1 1 1] rotate building
  (:Pressed
    (Variables|Default|SetShouldRotate? true))
  (:Released
    (Variables|Default|SetShouldRotate? false)))

(event Input|ActionEvents|InputActionFire
  (params (Key :type Key%20Structure :default "None"))
  (bind _playercharacter (Variables|Default|GetPlayerCharacter))
  (bind _returnvalue (Transformation|GetActorTransform _playercharacter))
  ;[1 1 1] Player fire
  (:Pressed
    (if (not (Variables|Default|GetIsBuilding?))
      (if (Variables|Default|GetCanFire?%20)
        (Variables|Default|SetCanFire?%20 false)
        (Utilities|FlowControl|Sequence
          (:then_0
            (Utilities|FlowControl|Delay 1.0)
            (Variables|Default|SetCanFire?%20 true))
          (:then_1
            (Game|SpawnActorfromClass "/Game/Blueprints/Turrets/TurretsProjectiles/BP_Projectile_fire.BP_Projectile_fire_C" (Math|Transform|MakeTransform (.location _returnvalue) (.rotation _returnvalue)) "Undefined" 0 0)
            (Animation|PlayAnimMontage _playercharacter "/Game/Blueprints/Characters/Player/Animation/Player_attack.Player_attack" 4.0 "LeftAction")))))))

(event Input|ActionEvents|InputActionTower1
  (params (Key :type Key%20Structure :default "None"))
  (:Released
    (if (>= (Variables|/Game/ThirdPersonBP/Blueprints/BP_Player.BP_Player_C|GetCoins (Variables|Default|GetPlayerCharacter)) 10)
      (Variables|Default|SetBuildClass "/Game/Blueprints/Turrets/BP_Tower_Normal.BP_Tower_Normal_C")
      (CallFunction|ToogleNewBuild) ; Has the toogle new building
    )))

(event Input|ActionEvents|InputActionTower2
  (params (Key :type Key%20Structure :default "None"))
  (:Released
    (if (>= (Variables|/Game/ThirdPersonBP/Blueprints/BP_Player.BP_Player_C|GetCoins (Variables|Default|GetPlayerCharacter)) 10)
      (Variables|Default|SetBuildClass "/Game/Blueprints/Turrets/BP_Tower_Fire.BP_Tower_Fire_C")
      (CallFunction|ToogleNewBuild) ; Has the toogle new building
    )))

(event Input|ActionEvents|InputActionUpgradeTower
  (params (Key :type Key%20Structure :default "None"))
  ;[1 1 1] Upgrade tower
  (:Released
    (bind _hitactor (CallFunction|UpgradeTower))
    (Variables|Default|SetTower_to_upgrade _hitactor)
    (Default|CallUpgradeTowerEvent)
    (EventDispatchers|BindEventtoUpgradeTowerEvent (delegate Custom|Upgrade_Tower))
    (Animation|PlayAnimMontage (Variables|Default|GetPlayerCharacter) "/Game/Blueprints/Characters/Player/Animation/Player_attack.Player_attack" 1.0 "RightAction")))

(event Input|ActionEvents|InputActionSellTower
  (params (Key :type Key%20Structure :default "None"))
  (bind _playercharacter (Variables|Default|GetPlayerCharacter))
  ;[1 1 1] Sell Tower
  (:Pressed
    (bind _hitactor (CallFunction|GetTower))
    (if (Variables|Default|GetIsTower?)
      (Actor|DestroyActor _hitactor)
      (Variables|/Game/ThirdPersonBP/Blueprints/BP_Player.BP_Player_C|SetCoins _playercharacter (+ (Variables|/Game/ThirdPersonBP/Blueprints/BP_Player.BP_Player_C|GetCoins _playercharacter) 10))
      (Audio|PlaySound2D "/Game/Sounds/sell.sell" 1.0 1.0 0.0 0 0))))

(event Input|ActionEvents|InputActionTower3
  (params (Key :type Key%20Structure :default "None"))
  (:Released
    (if (>= (Variables|/Game/ThirdPersonBP/Blueprints/BP_Player.BP_Player_C|GetCoins (Variables|Default|GetPlayerCharacter)) 10)
      (Variables|Default|SetBuildClass "/Game/Blueprints/Turrets/BP_Tower_Slow.BP_Tower_Slow_C")
      (CallFunction|ToogleNewBuild) ; Has the toogle new building
    )))

(event Input|KeyboardEvents|M
  (params (Key :type Key%20Structure :default "None"))
  ;[1 1 1] PauseMenu
  (:Pressed
    (CallFunction|ToogleMenu)))

(fn ConstructionScript)

(fn ToogleNewBuild
  (if (Variables|Default|GetIsBuilding?)
    (Variables|Default|SetIsBuilding? false)
    (Actor|DestroyActor (Variables|Default|GetBeing%20Build))
    (else
      (Variables|Default|SetIsBuilding? true)
      ;[1 1 1] Spawns the Item to be built next
      (CallFunction|SpawnBuildItem))))

(fn PositionPath
  (bind _being_build (Variables|Default|GetBeing%20Build))
  (bind (_bblockinghit _location _hitbuilditem_ _hititem) (CallFunction|CameraTrace)) ; Has Linetrace for building
  (LocalVariables|SetHitItem _hititem)
  (Utilities|FlowControl|Sequence
    (:then_0
      (CallFunction|MaterialCheck))
    (:then_1
      (LocalVariables|SetHit _location)
      (if _bblockinghit
        (if _hitbuilditem_
          (if (Variables|Default|GetMaterialCheck)
            (Actor|DestroyActor (Variables|Default|GetBeing%20Build))
            (Variables|Default|SetIsBuilding? false)
            (else
              (CallFunction|Snapto false (LocalVariables|GetHitItem) (LocalVariables|GetHit))
              (Variables|Default|SetMaterialCheck false)))
          (else
            (Transformation|SetActorLocation _being_build _location false false)
            (if (Variables|Default|GetShouldRotate?)
              (Class|Actor|AddActorWorldRotation _being_build "0,45.000000, 0"))))))))

(fn SpawnBuildItem
  (bind _returnvalue (Game|SpawnActorfromClass (Variables|Default|GetBuildClass) (Math|Transform|MakeTransform "0, 0, 0" "0, 0, 0" "3.000000,3.000000,3.000000") "AdjustIfPossibleButAlwaysSpawn" 0 0))
  (bind _output_get (Variables|Default|SetBeing%20Build _returnvalue))
  (Collision|SetCollisionEnabled (Variables|/Game/Blueprints/Turrets/BP_Tower.BP_Tower_C|GetStaticMesh _output_get) "NoCollision")
  (Rendering|Material|SetVectorParameterValueonMaterials (Variables|/Game/Blueprints/Turrets/BP_Tower.BP_Tower_C|GetTurretProj _output_get) "Tint" "0, 0,1.000000"))

(fn CameraTrace
  (bind _asbp_player (Utilities|Casting|CastToBP_Player (Game|GetPlayerCharacter 0))
    (:then
      (bind _outhit (Collision|LineTraceForObjects (Transformation|GetWorldLocation (Variables|/Game/ThirdPersonBP/Blueprints/BP_Player.BP_Player_C|GetFollowCamera _asbp_player)) (+ (Transformation|GetWorldLocation (Variables|/Game/ThirdPersonBP/Blueprints/BP_Player.BP_Player_C|GetFollowCamera _asbp_player)) (* (Math|Vector|GetForwardVector (Variables|/Game/ThirdPersonBP/Blueprints/BP_Player.BP_Player_C|GetFollowCamera _asbp_player)) 4e+03)) (Utilities|Array|MakeArray "ObjectTypeQuery7" "ObjectTypeQuery8") false 0 "None")))
    (:CastFailed
      _))
  (return (.bBlockingHit (Collision|BreakHitResult _outhit)) (.Location (Collision|BreakHitResult _outhit)) (.bSuccess (Utilities|Casting|CastToBP_Tower (.HitActor (Collision|BreakHitResult _outhit)))) (.AsBP%20Tower (Utilities|Casting|CastToBP_Tower (.HitActor (Collision|BreakHitResult _outhit))))))

(fn Snapto
  (params (PlaceTurret? :type Boolean) (SnapTo :type Actor%20Object%20Reference) (Hit :type Vector) (NewParam1 :type Actor%20Object%20Reference))
  (bind _returnvalue (Transformation|GetActorTransform SnapTo))
  (bind _returnvalue_2 (Transformation|GetActorTransform SnapTo))
  (bind _being_build (Variables|Default|GetBeing%20Build))
  (bind _returnvalue_3 (Math|Transform|InverseTransformLocation _returnvalue_2 Hit))
  (bind (_location _rotation) (Math|Transform|BreakTransform _returnvalue))
  (Math|Float|CompareFloat (Math|Float|Absolute(Float) (.x _returnvalue_3)) (Math|Float|Absolute(Float) (.y _returnvalue_3))
    (:>
      (LocalVariables|Setx_offset (* (Math|Float|Sign(Float) (.x _returnvalue_3)) (LocalVariables|GetOffset_amount))))
    (:==
      (LocalVariables|Sety_offset (* (Math|Float|Sign(Float) (.y _returnvalue_3)) (LocalVariables|GetOffset_amount)) :!label _label))
    (:<
      (goto _label)))
  (Transformation|SetActorTransform _being_build (Math|Transform|MakeTransform _location _rotation "3.000000,3.000000,3.000000"))
  (Transformation|AddActorLocalOffset _being_build (Math|Vector|MakeVector (LocalVariables|Getx_offset) (LocalVariables|Gety_offset) 0.0) false false))

(fn UpgradeTower
  (bind _playercharacter (Variables|Default|GetPlayerCharacter))
  (bind _hitactor (CallFunction|GetTower))
  (bind _asbp_tower (Utilities|Casting|CastToBP_Tower _hitactor))
  (if (>= (Variables|/Game/ThirdPersonBP/Blueprints/BP_Player.BP_Player_C|GetCoins _playercharacter) (* (Variables|Default|GetUpgradeFee) (Variables|/Game/Blueprints/Turrets/BP_Tower.BP_Tower_C|GetTower_Level _asbp_tower)))
    (if (<= (+ (Variables|/Game/Blueprints/Turrets/BP_Tower.BP_Tower_C|GetTower_Level _asbp_tower) 1) 3)
      (Utilities|FlowControl|Sequence
        (:then_0
          (Variables|/Game/ThirdPersonBP/Blueprints/BP_Player.BP_Player_C|SetCoins _playercharacter (- (Variables|/Game/ThirdPersonBP/Blueprints/BP_Player.BP_Player_C|GetCoins _playercharacter) (* (Variables|Default|GetUpgradeFee) (Variables|/Game/Blueprints/Turrets/BP_Tower.BP_Tower_C|GetTower_Level _asbp_tower)))))
        (:then_1
          (Variables|/Game/Blueprints/Turrets/BP_Tower.BP_Tower_C|SetTower_Level _asbp_tower (+ (Variables|/Game/Blueprints/Turrets/BP_Tower.BP_Tower_C|GetTower_Level _asbp_tower) 1))
          (Audio|PlaySound2D "/Game/Sounds/build.build" 1.0 1.0 0.0 0 0)
          (return _asbp_tower (Variables|/Game/Blueprints/Turrets/BP_Tower.BP_Tower_C|GetTower_Level _asbp_tower)))))))

(fn MaterialCheck
  (bind _being_build (Variables|Default|GetBeing%20Build))
  (bind _playercharacter (Variables|Default|GetPlayerCharacter))
  (bind _returnvalue (Transformation|GetActorLocation _being_build))
  (bind _outhit (Collision|LineTraceForObjects (Math|Vector|MakeVector (.x _returnvalue) (.y _returnvalue) (.z _returnvalue)) (+ (Math|Vector|MakeVector (.x _returnvalue) (.y _returnvalue) (.z _returnvalue)) "0, 0,-100.000000") (Utilities|Array|MakeArray "ObjectTypeQuery7") false 0 "None" true "(R=1.000000,G=0.000000,B=0.000000,A=1.000000)" "(R=0.000000,G=1.000000,B=0.000000,A=1.000000)" 1.0))
  (bind _output_get (Variables|Default|SetTakeBuildFee? (.bBlockingHit (Collision|BreakHitResult _outhit))))
  (Utilities|Casting|CastToBP_BuildLocation (.HitActor (Collision|BreakHitResult _outhit)))
  (Variables|Default|SetMaterialCheck true)
  (if _output_get
    (if (Variables|Default|GetClickToPlace)
      (Variables|/Game/ThirdPersonBP/Blueprints/BP_Player.BP_Player_C|SetCoins _playercharacter (- (Variables|/Game/ThirdPersonBP/Blueprints/BP_Player.BP_Player_C|GetCoins _playercharacter) 10)))))

(fn ToogleMenu
  (bind _aswidget_ui (Utilities|Casting|CastToWidget_UI (Variables|/Game/Blueprints/GameSettings/NewGameMode.NewGameMode_C|GetUserUI (Variables|Default|GetGameMode))))
  (LocalVariables|SetUserUI _aswidget_ui)
  (if (Variables|Default|GetEscapePressed?)
    (Variables|Default|SetEscapePressed? false)
    (Variables|Default|SetbShowMouseCursor false)
    (Widget|SetVisibility (LocalVariables|GetUserUI) "Visible")
    (Widget|SetVisibility (Variables|Default|GetPauseUI) "Hidden")
    (Game|SetGamePaused false)
    (else
      (Variables|Default|SetEscapePressed? true)
      (Variables|Default|SetbShowMouseCursor true)
      (Widget|SetVisibility (LocalVariables|GetUserUI) "Hidden")
      (bind _returnvalue (UserInterface|CreateWidget "/Game/Blueprints/UI/WG_Pause.WG_Pause_C"))
      (bind _output_get (Variables|Default|SetPauseUI _returnvalue))
      (UserInterface|Viewport|AddtoViewport _output_get 0)
      (Game|SetGamePaused true))))

(fn GetTower
  (bind _asbp_player (Utilities|Casting|CastToBP_Player (Game|Player|GetPlayerPawn 0)))
  (bind (_outhit _returnvalue) (Collision|LineTraceForObjects (Transformation|GetWorldLocation (Variables|/Game/ThirdPersonBP/Blueprints/BP_Player.BP_Player_C|GetFollowCamera _asbp_player)) (+ (Transformation|GetWorldLocation (Variables|/Game/ThirdPersonBP/Blueprints/BP_Player.BP_Player_C|GetFollowCamera _asbp_player)) (* (Math|Vector|GetForwardVector (Variables|/Game/ThirdPersonBP/Blueprints/BP_Player.BP_Player_C|GetFollowCamera _asbp_player)) 5e+03)) (Utilities|Array|MakeArray "ObjectTypeQuery8") false 0 "None"))
  (Variables|Default|SetIsTower? _returnvalue)
  (return (.HitActor (Collision|BreakHitResult _outhit))))