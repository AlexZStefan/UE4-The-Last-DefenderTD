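; BP_Tower is an upgradeable defense turret that targets and shoots living BP_Enemy actors in range.
; Each tick it picks a visible target via sphere overlap, measuring distance against its owner cast to BP_Enemy, then rotates with clamped pitch.
; It spawns projectiles once cooldown and a dot-product facing check pass; a near-identical Slow event is uncalled here.
; A player controller upgrade event applies scale and fire-interval changes based on TowerLevel.
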(event Custom|Slow
  ;[1 1 1] Projectile spawner
  (Variables|Default|SetTimeOfLastFire (Utilities|Time|GetGameTimeinSeconds))
  (Collision|SphereTraceByChannel "0, 0, 0" "0, 0, 0" 0.0 "TraceTypeQuery2" false 0 "None")
  (Audio|PlaySoundatLocation "/Game/Sounds/TestSound.TestSound" "0, 0, 0" "0, 0, 0" 1.0 1.0 0.0 0 0 0)
  (Game|SpawnActorfromClass (Variables|Default|GetProjectile_type) (Transformation|GetSocketTransform (Variables|Default|GetTurretProj) "FireGun" "RTS_World") "Undefined" 0 0)
  (Utilities|FlowControl|Delay 0.2))

(event Custom|Fire
  ;[1 1 1] Projectile spawner
  (Variables|Default|SetTimeOfLastFire (Utilities|Time|GetGameTimeinSeconds))
  (Collision|SphereTraceByChannel "0, 0, 0" "0, 0, 0" 0.0 "TraceTypeQuery1" false 0 "None")
  (Audio|PlaySoundatLocation "/Game/Sounds/TestSound.TestSound" "0, 0, 0" "0, 0, 0" 1.0 1.0 0.0 0 0 0)
  (Game|SpawnActorfromClass (Variables|Default|GetProjectile_type) (Transformation|GetSocketTransform (Variables|Default|GetTurretProj) "FireGun" "RTS_World") "Undefined" 0 0)
  (Utilities|FlowControl|Delay 0.2))

(event Custom|Tower_Upgrade
  (CallFunction|Upgrade))

(event Custom|Upgrade
  (bind _tower_level (Variables|Default|GetTower_Level))
  ;[1 1 1] Set the proprieties for when tower is upgraded
  (Utilities|FlowControl|Sequence
    (:then_0
      (if (== _tower_level 1)
        (Variables|Default|SetRateOfFire (Variables|Default|GetRateOfFire))))
    (:then_1
      (if (== _tower_level 2)
        (Transformation|SetActorScale3D "4.000000,4.000000,4.000000")
        (Variables|Default|SetRateOfFire (- (Variables|Default|GetRateOfFire) 0.2))))
    (:then_2
      (if (== _tower_level 3)
        (Transformation|SetActorScale3D "5.000000,5.000000,5.000000")
        (Variables|Default|SetRateOfFire (- (Variables|Default|GetRateOfFire) 0.5))))))

(event EventBeginPlay
  (Utilities|FlowControl|Sequence
    (:then_0
      (bind _asbp_player (Utilities|Casting|CastToBP_Player (Game|Player|GetPlayerPawn 0)))
      (Variables|Default|SetPlayer _asbp_player))
    (:then_1
      (bind _asbp_enemy (Utilities|Casting|CastToBP_Enemy (Components|GetOwner)))
      (Variables|Default|SetEnemy _asbp_enemy))
    (:then_2
      (bind _asnew_player_controller (Utilities|Casting|CastToNewPlayerController (Game|GetPlayerController 0)))
      (bind _output_get (Variables|Default|SetPlayerController _asnew_player_controller))
      (EventDispatchers|BindEventtoUpgradeTowerEvent _output_get (delegate Custom|Tower_Upgrade)))))

(event EventTick
  (params (DeltaSeconds :type Float%20%28single-precision%29))
  ;[1 1 1] Turret Movement and Fire
  (CallFunction|FindTarget)
  (Variables|Default|GetTarget
    (:then
      (CallFunction|UpdateTurretRotation DeltaSeconds)
      (CallFunction|UpdateFire))
    (:else)))

(fn ConstructionScript)

(fn FindTarget
  (LocalVariables|SetRange_to_target%28Local%29 (+ (Variables|Default|GetTurret_Range) 1.0))
  ;[1 1 1] Checks for enemies within range - adds them to array
  (bind _outactors (Collision|SphereOverlapActors (Transformation|GetActorLocation) (Variables|Default|GetTurret_Range) (Utilities|Array|MakeArray "ObjectTypeQuery3") "/Game/Blueprints/ThirdPersonBP/Blueprints/BP_Enemy.BP_Enemy_C"))
  (Utilities|FlowControl|Sequence
    (:then_1
      (for _array_element _outactors
        (if (> (Variables|/Game/Blueprints/ThirdPersonBP/Blueprints/BP_Enemy.BP_Enemy_C|GetHealth (.AsBP%20Enemy (Utilities|Casting|CastToBP_Enemy _array_element))) 0.0)
          ;[1 1 1] Gets distance from turret to enemy - assigns to current distance
          (bind _output_get (LocalVariables|SetCurrentTarget%28local%29 _array_element))
          ;[1 1 1] Checks the enemy is within range of turret - or - if target is not valid
          (bind _output_get_2 (LocalVariables|SetCurrent_Distance%20%28local%29 (Transformation|GetDistanceTo _output_get (Variables|Default|GetEnemy))))
          (if (or (<= _output_get_2 (LocalVariables|GetRange_to_target%28Local%29)) (not (Utilities|IsValid (LocalVariables|GetBest_target%28Local%29))))
            (bind _result (CallFunction|HasLineOfSight (Transformation|GetWorldLocation (Variables|Default|GetTurretProj)) (Transformation|GetActorLocation (LocalVariables|GetCurrentTarget%28local%29)) (Utilities|Array|MakeArray self (LocalVariables|GetCurrentTarget%28local%29))))
            (if _result
              (LocalVariables|SetBest_target%28Local%29 (LocalVariables|GetCurrentTarget%28local%29))
              (LocalVariables|SetRange_to_target%28Local%29 (LocalVariables|GetCurrent_Distance%20%28local%29))))))
      (Variables|Default|SetTarget (LocalVariables|GetBest_target%28Local%29)))))

(fn UpdateTurretRotation
  (params (DeltaSeconds :type Float%20%28single-precision%29))
  (bind _turretproj (Variables|Default|GetTurretProj))
  (bind _output_get (Variables|Default|SetNewRotatation (Class|KismetMathLibrary|RInterptoConstant (Transformation|GetWorldRotation _turretproj) (Math|Rotator|FindLookatRotation (Transformation|GetWorldLocation _turretproj) (Transformation|GetActorLocation (Variables|Default|GetTarget))) DeltaSeconds (Variables|Default|GetTurretRotationSpeed))))
  ;[1 1 1] rotates the TurretBarrel
  (Transformation|SetWorldRotation (Variables|Default|GetTurretProj) (Math|Rotator|MakeRotator (.roll _output_get) (Math|Float|ClampAngle (.pitch _output_get) -45.0 0.0) (.yaw _output_get)) false false))

(fn UpdateFire
  (if (> (- (Utilities|Time|GetGameTimeinSeconds) (Variables|Default|GetTimeOfLastFire)) (Variables|Default|GetRateOfFire)) ; Fire Cooled down?
    (if (>= (Math|Vector|DotProduct (Math|Vector|GetUnitDirection(Vector) (Transformation|GetWorldLocation (Variables|Default|GetTurretProj)) (Transformation|GetActorLocation (Variables|Default|GetTarget))) (Math|Vector|GetForwardVector (Variables|Default|GetTurretProj))) 0.95) ; Is turret facing the target?
      (CallFunction|Fire))))