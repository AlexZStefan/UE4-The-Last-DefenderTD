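; BP_Projectile_fire is a turret projectile that hits enemies, passing damage, slow and fire values to them.
; When its Sphere overlaps a BP_Enemy, it calls TakeDamage on that enemy and destroys itself after a zero-length delay.
; BeginPlay also tries to cast the player character to BP_Enemy and store it as Enemy, which the overlap logic does not use.
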(event OnComponentBeginOverlap(Sphere)
  (params (OverlappedComponent :type Primitive%20Component%20Object%20Reference) (OtherActor :type Actor%20Object%20Reference) (OtherComp :type Primitive%20Component%20Object%20Reference) (OtherBodyIndex :type Integer) (bFromSweep :type Boolean) (SweepResult :type Hit%20Result%20Structure%20%28by%20ref%29))
  (bind _asbp_enemy (Utilities|Casting|CastToBP_Enemy OtherActor))
  (Default|TakeDamage _asbp_enemy (Variables|Default|GetProjectile_Damage) (Variables|Default|GetSlow) (Variables|Default|GetFire))
  (Utilities|FlowControl|Delay 0.0)
  (Actor|DestroyActor))

(event EventBeginPlay
  (bind _asbp_enemy (Utilities|Casting|CastToBP_Enemy (Game|GetPlayerCharacter 0)))
  (Variables|Default|SetEnemy _asbp_enemy))

(event Collision|EventActorBeginOverlap
  (params (OtherActor :type Actor%20Object%20Reference)))

(event EventTick
  (params (DeltaSeconds :type Float%20%28single-precision%29)))

(fn ConstructionScript)