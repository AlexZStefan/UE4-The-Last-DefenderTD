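; Track generator Blueprint that builds a closed-loop road from spline meshes along an editable spline in its construction script.
; It counts the spline points, then trims or pads RoadDataArray with defaults to match, preserving existing per-point entries.
; Each point gets a spline mesh to the next, wrapping via modulo, with tangents from the spline and bank, width and thickness interpolated between both points' data.
; Collision is toggled by a flag.
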(event EventBeginPlay)

(event Collision|EventActorBeginOverlap
  (params (OtherActor :type Actor%20Object%20Reference)))

(event EventTick
  (params (DeltaSeconds :type Float%20%28single-precision%29)))

(fn ConstructionScript
  (Utilities|FlowControl|Sequence
    (:then_0
      (|Storesplinepoints))
    (:then_1
      (|BuildRoadDataarray))
    (:then_2
      (for _index (range 0 (- (Variables|Default|GetNumber%20of%20spline%20points) 1))
        (CallFunction|BuildTrackElement _index (Variables|Default|GetRoadMesh))))
    (:then_3)))

(fn BuildTrackElement
  (params (LoopIndex :type Integer) (TrackElementMesh :type Static%20Mesh%20Object%20Reference))
  (LocalVariables|SetL_currentLoopIndex LoopIndex)
  (LocalVariables|SetL_NextLoopIndex (Math|Integer|%(Integer) (+ LoopIndex 1) (Variables|Default|GetNumber%20of%20spline%20points)))
  (LocalVariables|SetL_TrackElementMesh TrackElementMesh)
  (Utilities|FlowControl|Sequence
    (:then_0
      (LocalVariables|SetL_startLocation (.Location (Spline|GetLocationandTangentatSplinePoint (Variables|Default|GetSpline) (LocalVariables|GetL_currentLoopIndex) "Local")))
      (LocalVariables|SetL_startTangent (.Tangent (Spline|GetLocationandTangentatSplinePoint (Variables|Default|GetSpline) (LocalVariables|GetL_currentLoopIndex) "Local")))
      (LocalVariables|SetL_EndLocation (.Location (Spline|GetLocationandTangentatSplinePoint (Variables|Default|GetSpline) (LocalVariables|GetL_NextLoopIndex) "Local")))
      (LocalVariables|SetL_EndTangent (.Tangent (Spline|GetLocationandTangentatSplinePoint (Variables|Default|GetSpline) (LocalVariables|GetL_NextLoopIndex) "Local")))
      (LocalVariables|SetL_StartRoll (.trackbank (Utilities|Array|Get(acopy) (Variables|Default|GetRoadDataArray) (LocalVariables|GetL_currentLoopIndex))))
      (LocalVariables|SetL_StartScale (Math|Vector2D|MakeVector2D (.trackwidth (Utilities|Array|Get(acopy) (Variables|Default|GetRoadDataArray) (LocalVariables|GetL_currentLoopIndex))) (.trachthickness (Utilities|Array|Get(acopy) (Variables|Default|GetRoadDataArray) (LocalVariables|GetL_currentLoopIndex)))))
      (LocalVariables|SetL_EndRoll (.trackbank (Utilities|Array|Get(acopy) (Variables|Default|GetRoadDataArray) (LocalVariables|GetL_NextLoopIndex))))
      (LocalVariables|SetL_EndScale (Math|Vector2D|MakeVector2D (.trackwidth (Utilities|Array|Get(acopy) (Variables|Default|GetRoadDataArray) (LocalVariables|GetL_NextLoopIndex))) (.trachthickness (Utilities|Array|Get(acopy) (Variables|Default|GetRoadDataArray) (LocalVariables|GetL_NextLoopIndex))))))
    (:then_1
      (bind _returnvalue (AddComponent|AddSplineMeshComponent false))
      (LocalVariables|SetL_CurrentSplineMesh _returnvalue)
      (Components|StaticMesh|SetStaticMesh (LocalVariables|GetL_CurrentSplineMesh) (LocalVariables|GetL_TrackElementMesh))
      (SplineMesh|SetStartandEnd (LocalVariables|GetL_CurrentSplineMesh) (LocalVariables|GetL_startLocation) (LocalVariables|GetL_startTangent) (LocalVariables|GetL_EndLocation) (LocalVariables|GetL_EndTangent) true :!class /Script/Engine.SplineMeshComponent)
      (Class|SplineMeshComponent|SetStartRoll (LocalVariables|GetL_CurrentSplineMesh) (LocalVariables|GetL_StartRoll) true)
      (Class|SplineMeshComponent|SetEndRoll (LocalVariables|GetL_CurrentSplineMesh) (LocalVariables|GetL_EndRoll) true)
      (SplineMesh|SetStartScale (LocalVariables|GetL_CurrentSplineMesh) (LocalVariables|GetL_StartScale) true :!class /Script/Engine.SplineMeshComponent)
      (SplineMesh|SetEndScale (LocalVariables|GetL_CurrentSplineMesh) (LocalVariables|GetL_EndScale) true :!class /Script/Engine.SplineMeshComponent)
      (Collision|SetCollisionEnabled (LocalVariables|GetL_CurrentSplineMesh) (select (Variables|Default|GetCollision) "QueryAndPhysics" "NoCollision")))))